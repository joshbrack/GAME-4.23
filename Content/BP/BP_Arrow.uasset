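; BP_Arrow is an arrow actor that detects whether it struck an archery target from the front or the back.
; When the Arrowhead overlaps a BP_ArcheryTarget, the dot product of both forward vectors decides the side.
; Front hits print a message and call TargetHasBeenShot on the target, while back hits only print a message.
; The Cylinder hit event is empty and the destroy-arrow logic is disconnected.
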(event OnComponentHit(Cylinder)
  (params (HitComponent :type Primitive%20Component%20Object%20Reference) (OtherActor :type Actor%20Object%20Reference) (OtherComp :type Primitive%20Component%20Object%20Reference) (NormalImpulse :type Vector :default "0, 0, 0") (Hit :type Hit%20Result%20Structure%20%28by%20ref%29)))

(event OnComponentBeginOverlap(Arrowhead)
  (params (OverlappedComponent :type Primitive%20Component%20Object%20Reference) (OtherActor :type Actor%20Object%20Reference) (OtherComp :type Primitive%20Component%20Object%20Reference) (OtherBodyIndex :type Integer) (bFromSweep :type Boolean) (SweepResult :type Hit%20Result%20Structure%20%28by%20ref%29))
  ;[1 1 1] has arrow hit front of target
  (bind _asbp_archery_target (Utilities|Casting|CastToBP_ArcheryTarget OtherActor))
  (if (<= (Math|Vector|DotProduct (Transformation|GetActorForwardVector) (Transformation|GetActorForwardVector _asbp_archery_target)) 0.0)
    (Development|PrintString "shot target in front" true true "(R=1.000000,G=0.957199,B=0.034897,A=1.000000)")
    (Default|TargetHasBeenShot _asbp_archery_target)
    (else
      (Development|PrintString "shot target in back" true true "(R=1.000000,G=0.282183,B=0.192456,A=1.000000)"))))

(fn ConstructionScript)
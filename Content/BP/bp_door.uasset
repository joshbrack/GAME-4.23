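; Sliding double door that opens either from an external trigger or with a player's key.
; The activatedoors event, commented as target-driven, opens it directly without checking or clearing the lock.
; Box overlap by a BP-CHAR holding a key unlocks a locked door, uses the key and opens it; overlap does nothing when already unlocked.
; Two timelines lerp the left and right panels' relative locations, with no closing logic.
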(event OnComponentBeginOverlap(Box)
  (params (OverlappedComponent :type Primitive%20Component%20Object%20Reference) (OtherActor :type Actor%20Object%20Reference) (OtherComp :type Primitive%20Component%20Object%20Reference) (OtherBodyIndex :type Integer) (bFromSweep :type Boolean) (SweepResult :type Hit%20Result%20Structure%20%28by%20ref%29))
  ;[1 1 1] open door with key
  (bind _asbp_char (Utilities|Casting|CastToBP-CHAR OtherActor))
  (if (Variables|Default|Getlocked) ; is the door locked
    (if (> (Variables|/Game/BP/BP-CHAR.BP-CHAR_C|Getkeys _asbp_char) 0) ; does player have key
      (Variables|Default|Setlocked false) ; unlock door
      (Default|UseKey _asbp_char)
      (CallFunction|OpenDoor))))

(event Custom|activate%20doors
  ;[1 1 1] open door with target
  (CallFunction|OpenDoor))

(event Custom|open%20door
  ;[1 1 1] animation
  (Utilities|FlowControl|Sequence
    (:then_0
      (bind _newtrack_0 (Timeline|Timeline_2 Play)
        (:Update
          (Transformation|SetRelativeLocation (Variables|Default|Getleft%20door) (Math|Vector|Lerp(Vector) "0.006267,141.906311,-92.529984" "-0.000000,11.790773,-92.529984" _newtrack_0) false false))))
    (:then_1
      (bind _newtrack_0_2 (Timeline|Timeline_3 Play)
        (:Update
          (Transformation|SetRelativeLocation (Variables|Default|Getright%20door) (Math|Vector|Lerp(Vector) "-0.002982,-247.710297,-92.529984" "-0.000118,-109.122757,-92.529984" _newtrack_0_2) false false))))))

(fn ConstructionScript)
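; BP_PRESSUREPAD is a pressure plate that tracks whether it is pressed in an IsActive flag, which comments indicate is meant for opening and closing a door.
; Its COLLISION overlaps react to physics-simulating components or actors of a specific class.
; Begin overlap sets the flag and gives PRESSUREPLATE the Mcoin material; end overlap clears it and applies Black.
; Overlaps are not counted, so any qualifying exit deactivates the pad.
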(event OnComponentBeginOverlap(COLLISION)
  (params (OverlappedComponent :type Primitive%20Component%20Object%20Reference) (OtherActor :type Actor%20Object%20Reference) (OtherComp :type Primitive%20Component%20Object%20Reference) (OtherBodyIndex :type Integer) (bFromSweep :type Boolean) (SweepResult :type Hit%20Result%20Structure%20%28by%20ref%29))
  ;[1 1 1] open door when pressed
  (if (or (Physics|IsSimulatingPhysics OtherComp "None") (== (Utilities|GetClass OtherActor) 0))
    (Variables|Default|Setis%20active? true)
    (Rendering|Material|SetMaterial (Variables|Default|GetPRESSURE%20PLATE) 0 "/Game/MATS/m-coin.m-coin")))

(event OnComponentEndOverlap(COLLISION)
  (params (OverlappedComponent :type Primitive%20Component%20Object%20Reference) (OtherActor :type Actor%20Object%20Reference) (OtherComp :type Primitive%20Component%20Object%20Reference) (OtherBodyIndex :type Integer))
  ;[1 1 1] close door when released
  (if (or (Physics|IsSimulatingPhysics OtherComp "None") (== (Utilities|GetClass OtherActor) 0))
    (Variables|Default|Setis%20active? false)
    (Rendering|Material|SetMaterial (Variables|Default|GetPRESSURE%20PLATE) 0 "/Game/MATS/black.black")))

(event EventBeginPlay)

(event Collision|EventActorBeginOverlap
  (params (OtherActor :type Actor%20Object%20Reference)))

(event EventTick
  (params (DeltaSeconds :type Float%20%28single-precision%29)))

(fn ConstructionScript)